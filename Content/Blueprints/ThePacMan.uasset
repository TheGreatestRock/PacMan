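; Player Pac-Man Blueprint that handles scoring, lives and level end through actor overlaps.
; Frightened, living ghosts are killed on touch; other ghost contact costs a life and updates the UIPacMan widget, or opens the main menu when none remain.
; Eatables add score, with SuperPacGomme also frightening all ghosts.
; Touching the last Eatable, found by counting those in the level, plays the intermission sound and returns to the menu.
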(event `self.ReceiveActorBeginOverlap`
  (params (OtherActor :type "Actor Object Reference"))
  (bind _lives (`self.Lives`))
  (bind _score (`self.Score`))
  (`KismetSystemLibrary.PrintText` (`KismetTextLibrary.Conv_IntToText` _score))
  (bind _asghost (cast `Ghost` OtherActor)
    (:`then`
      (if (and (`Ghost.bIsFrightened` _asghost) (not (`Ghost.bIsDead` _asghost)))
        (`Ghost.SetDeadMode` _asghost)
        (`GameplayStatics.PlaySound2D` "/Game/Assets/sounds/eat_ghost.eat_ghost" 1.0 1.0 0.0 null null)
        (`Controller.StopMovement` (`AIBlueprintHelperLibrary.GetAIController` _asghost))
        (elif (> _lives 0)
          (bind _result (`/Engine/EditorBlueprintResources/StandardMacros.DecrementInt` _lives)
            (:`  `
              (bind _output_get (set `self.Lives` _result))
              (`KismetSystemLibrary.PrintText` (`KismetTextLibrary.Conv_IntToText` _output_get))
              (bind _foundwidgets (`WidgetBlueprintLibrary.GetAllWidgetsOfClass` "/Game/UI/UIPacMan.UIPacMan_C"))
              (`/Game/UI/UIPacMan.loselife` _foundwidgets)
              (`GameplayStatics.PlaySound2D` "/Game/Assets/sounds/death_0.death_0" 1.0 1.0 0.0 null null)))
          (else
            (`GameplayStatics.PlaySound2D` "/Game/Assets/sounds/death_0.death_0" 1.0 1.0 0.0 null null)
            (`GameplayStatics.PlaySound2D` "/Game/Assets/sounds/death_1.death_1" 1.0 1.0 0.0 null null)
            (`GameplayStatics.PlaySound2D` "/Game/Assets/sounds/death_1.death_1" 1.0 1.0 0.0 null null)
            (`GameplayStatics.OpenLevelBySoftObjectPtr` "/Game/Levels/LVPM_MainMenu.LVPM_MainMenu")))))
    (:`CastFailed`
      (cast `Eatable` OtherActor)
      (bind _outactors (`GameplayStatics.GetAllActorsOfClass` "/Script/PacMan.Eatable"))
      (bind _returnvalue (`KismetArrayLibrary.Array_Length` _outactors))
      (`KismetSystemLibrary.PrintText` (`KismetTextLibrary.Conv_IntToText` _returnvalue))
      (if (<= _returnvalue 1)
        (`GameplayStatics.PlaySound2D` "/Game/Assets/sounds/intermission.intermission" 1.0 1.0 0.0 null null)
        (`GameplayStatics.OpenLevelBySoftObjectPtr` "/Game/Levels/LVPM_MainMenu.LVPM_MainMenu")
        (else
          (cast `SuperPacGomme` OtherActor
            (:`then`
              (set `self.Score` (+ _score 50))
              (bind _outactors_2 (`GameplayStatics.GetAllActorsOfClass` "/Script/PacMan.Ghost"))
              (`Ghost.SetFrightenMode` _outactors_2))
            (:`CastFailed`
              (set `self.Score` (+ _score 10)))))))))

(event `self.ReceiveBeginPlay`
  (bind _returnvalue (`AddComponent|NODE_AddAudioComponent-0`))
  (add `AudioComponent.OnAudioFinished` _returnvalue (delegate `OnAudioFinished_Événement`)))

(event `OnAudioFinished_Événement`)

(fn `UserConstructionScript`)
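; Inky is a ghost Blueprint, apparently for a Pac-Man style game, that handles the ghost's sprite appearance.
; It sets the normal Inky sprite on BeginPlay, then reselects the sprite every Tick from the IsDead and IsFrightened flags.
; Dead takes priority over frightened, and the normal sprite is the fallback.
; The graph only reads these flags, and its overlap event and construction script are empty.
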(event `self.ReceiveBeginPlay`
  (`PaperSpriteComponent.SetSprite` (`self.Inky_Sprite`) "/Game/Textures/Sprites/Inky_Sprite.Inky_Sprite"))

(event `self.ReceiveActorBeginOverlap`
  (params (OtherActor :type "Actor Object Reference")))

(event `self.ReceiveTick`
  (params (DeltaSeconds :type "Float (single-precision)"))
  (bind _inky_sprite (`self.Inky_Sprite`))
  (bind _bisdead (`self.bIsDead`))
  (if (and (`self.bIsFrightened`) (not _bisdead))
    (`PaperSpriteComponent.SetSprite` _inky_sprite "/Game/Textures/Sprites/frightened.frightened")
    (elif _bisdead
      (`PaperSpriteComponent.SetSprite` _inky_sprite "/Game/Textures/Sprites/ded.ded")
      (else
        (`PaperSpriteComponent.SetSprite` _inky_sprite "/Game/Textures/Sprites/Inky_Sprite.Inky_Sprite")))))

(fn `UserConstructionScript`)